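; BP_Trash is a trash pickup actor with a TrashType enum and a Cube mesh.
; Interact prints the picked-up trash type and calls DestoyItem, which plays a timeline that drives the cube's scale, then destroys the actor when it finishes.
; GetStaticMesh exposes the cube's static mesh to callers.
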(event Custom|DestoyItem
  (bind _newtrack_0 (Timeline|Timeline_0 Play)
    (:Update
      (Transformation|SetRelativeScale3D (Variables|Default|GetCube) _newtrack_0))
    (:Finished
      (Actor|DestroyActor))))

(fn ConstructionScript)

(fn GetStaticMesh
  (return (Variables|/Script/Engine.StaticMeshComponent|GetStaticMesh (Variables|Default|GetCube))))

(fn Interact
  (Development|PrintString (Utilities|String|Append "Picked up: " (Utilities|String|EnumtoString (Variables|Default|GetTrashType))))
  (CallFunction|DestoyItem)
  (return))