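; Conveyor belt actor that carries objects along the direction of its Arrow component.
; Each Tick it gathers the actors overlapping its Box and keeps only those implementing BPI_Interact.
; It shifts each one by the Arrow's forward vector scaled by Speed and delta time, using an unswept world offset, so movement ignores collision.
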(event EventBeginPlay)

(event Collision|EventActorBeginOverlap
  (params (OtherActor :type Actor%20Object%20Reference)))

(event EventTick
  (params (DeltaSeconds :type Float%20%28single-precision%29))
  (for _array_element (Collision|GetOverlappingActors (Variables|Default|GetBox) 0 :!class /Script/Engine.PrimitiveComponent)
    (if (Utilities|DoesObjectImplementInterface _array_element "/Game/Blueprints/BPI_Interact.BPI_Interact_C")
      (Transformation|AddActorWorldOffset _array_element (* (Math|Vector|GetForwardVector (Variables|Default|GetArrow)) (* DeltaSeconds (Variables|Default|GetSpeed)))))))

(fn ConstructionScript)